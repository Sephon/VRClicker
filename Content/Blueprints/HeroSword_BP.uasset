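; Grabbable hero sword actor that BP_MotionController picks up and that damages whatever it hits.
; Pickup turns off mesh physics, snaps the root to the supplied component, then rotates and nudges the mesh to align it.
; Drop re-enables physics and detaches the sword in place.
; On hit, it applies fixed point damage and pushes the struck component with an impulse equal to the unscaled hit normal.
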(event EventBeginPlay)

(event Collision|EventActorBeginOverlap
  (params (OtherActor :type Actor%20Object%20Reference)))

(event EventTick
  (params (DeltaSeconds :type Float%20%28single-precision%29)))

(event EventPickup
  (params (AttachTo :type Scene%20Component%20Object%20Reference))
  (Physics|SetSimulatePhysics (Variables|Default|GetStaticMesh) false)
  (Transformation|AttachComponentToComponent (VehicleSound|GetRootComponent) AttachTo "None" "SnapToTarget" "SnapToTarget" "SnapToTarget" false)
  (Transformation|AddLocalRotation (Variables|Default|GetStaticMesh) "0,90.000000, 0" false false)
  (Transformation|AddLocalOffset (Variables|Default|GetStaticMesh) "0,2.000000, 0" false false))

(event EventDrop
  (Physics|SetSimulatePhysics (Variables|Default|GetStaticMesh) true)
  (Transformation|DetachFromActor "KeepWorld" "KeepWorld" "KeepWorld"))

(event Collision|EventHit
  (params (MyComp :type Primitive%20Component%20Object%20Reference) (Other :type Actor%20Object%20Reference) (OtherComp :type Primitive%20Component%20Object%20Reference) (bSelfMoved :type Boolean) (HitLocation :type Vector :default "0, 0, 0") (HitNormal :type Vector :default "0, 0, 0") (NormalImpulse :type Vector :default "0, 0, 0") (Hit :type Hit%20Result%20Structure%20%28by%20ref%29))
  (Game|Damage|ApplyPointDamage Other 1e+02 (.ImpactPoint (Collision|BreakHitResult Hit)) Hit 0 self)
  (Physics|AddImpulseatLocation OtherComp HitNormal HitLocation "None"))

(fn ConstructionScript)