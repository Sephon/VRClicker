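; Destructible cube actor that reacts to hero sword strikes and explodes on point damage.
; Component hits from HeroSword_BP apply fixed point damage to the hit result's actor and spawn temporary debug text showing mass, velocity and damage.
; Receiving point damage plays a randomized explosion sound and spawns a short-lived explosion effect.
; Pickup-cube and impulse logic is left disconnected, and the mass-times-velocity calculation is unused.
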(event OnComponentHit(Destructible)
  (params (HitComponent :type Primitive%20Component%20Object%20Reference) (OtherActor :type Actor%20Object%20Reference) (OtherComp :type Primitive%20Component%20Object%20Reference) (NormalImpulse :type Vector :default "0, 0, 0") (Hit :type Hit%20Result%20Structure%20%28by%20ref%29))
  (bind (_bblockinghit _binitialoverlap _time _distance _location _impactpoint _normal _impactnormal _physmat _hitactor) (Collision|BreakHitResult Hit))
  (Utilities|Casting|CastToHeroSword_BP OtherActor)
  (bind _returnvalue (Game|Damage|ApplyPointDamage _hitactor 1e+02 _impactpoint Hit 0 0 "/Script/Engine.DamageType"))
  (bind _returnvalue_2 (Game|SpawnActorfromClass "/Script/Engine.TextRenderActor" (Math|Conversions|ToTransform(Vector) _impactpoint) "Undefined" 0 0))
  (Transformation|AddLocalRotation (Variables|/Script/Engine.Actor|GetRootComponent _returnvalue_2) "0,180.000000, 0" false false) ; Temporary rotation for readability
  (Rendering|Components|TextRender|SetText (Variables|/Script/Engine.TextRenderActor|GetTextRender _returnvalue_2) (Utilities|Text|ToText(String) (Utilities|String|BuildString(Float) (Utilities|String|BuildString(Float) (Utilities|String|BuildString(Float) "" "Mass:  " (Physics|GetMass OtherComp) ", ") "Velocity: " (Math|Vector|VectorLength (Transformation|GetVelocity OtherActor)) ", ") "Afflicated " _returnvalue " points of damage")))
  (Utilities|FlowControl|Delay 5.0)
  (Actor|DestroyActor _returnvalue_2)
  (Rendering|ToggleVisibility (Variables|/Script/Engine.Actor|GetRootComponent _returnvalue_2) true))

(event EventBeginPlay)

(event Collision|EventActorBeginOverlap
  (params (OtherActor :type Actor%20Object%20Reference)))

(event EventTick
  (params (DeltaSeconds :type Float%20%28single-precision%29)))

(event Game|Damage|EventPointDamage
  (params (Damage :type Float%20%28single-precision%29) (DamageType :type Damage%20Type%20Object%20Reference) (HitLocation :type Vector :default "0, 0, 0") (HitNormal :type Vector :default "0, 0, 0") (HitComponent :type Primitive%20Component%20Object%20Reference) (BoneName :type Name :default "None") (ShotFromDirection :type Vector :default "0, 0, 0") (InstigatedBy :type Controller%20Object%20Reference) (DamageCauser :type Actor%20Object%20Reference) (HitInfo :type Hit%20Result%20Structure%20%28by%20ref%29))
  (Audio|PlaySoundatLocation "/Game/StarterContent/Audio/Explosion01.Explosion01" HitLocation "0, 0, 0" (Math|Random|RandomFloatinRange 0.8 1.2) (Math|Random|RandomFloatinRange 0.5 1.5))
  (bind _returnvalue (Game|SpawnActorfromClass "/Game/StarterContent/Blueprints/Blueprint_Effect_Explosion.Blueprint_Effect_Explosion_C" (Transformation|GetActorTransform) "Undefined" 0 0))
  (Utilities|FlowControl|Delay 2.0)
  (Actor|DestroyActor _returnvalue) ; Cleanup explosion
)

(fn ConstructionScript)