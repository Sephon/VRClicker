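; StaticCannon is an actor that repeatedly fires Destructible_Cube actors from its own position.
; Tick feeds a Delay of the absolute SpawnDelay, which acts as a repeating timer, then spawns a cube at the cannon's transform regardless of collisions.
; A fixed world-space impulse, toward negative X and upward, hits both the cannon's StaticMesh and the cube's Destructible at the cannon's location.
; AddForce and attach nodes are left unconnected.
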(event EventBeginPlay)

(event Collision|EventActorBeginOverlap
  (params (OtherActor :type Actor%20Object%20Reference)))

(event EventTick
  (params (DeltaSeconds :type Float%20%28single-precision%29))
  (Utilities|FlowControl|Delay (Math|Float|Absolute(Float) (Variables|Default|GetSpawn_Delay)))
  (bind _returnvalue (Game|SpawnActorfromClass "/Game/Blueprints/Destructible_Cube.Destructible_Cube_C" (Transformation|GetActorTransform) "AlwaysSpawn" 0 0))
  (Physics|AddImpulseatLocation (Variables|Default|GetStaticMesh) "-50000.000000,0.000000,10000.000000" (Transformation|GetActorLocation) "None"))

(fn ConstructionScript)